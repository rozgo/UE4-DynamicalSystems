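; BP_MicroAreaExit is an interactable exit for a micro world, marked by a text render.
; Its BP_Interactable events drive it: interaction calls the exit function on MicroWorldOwner, which handles the actual exit.
; Hover and unhover switch the text between highlight and normal colors, and the construction script applies the normal color initially.
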(event `self.BP_Interactable.OnInteracted`
  (params (Selector :type "/DynamicalSystems/Blueprints/BP_InteractableSelector Object Reference"))
  (`/DynamicalSystems/Blueprints/BP_MicroArea.OnMiroWorldExit` (`self.MicroWorldOwner`)))

(event `self.BP_Interactable.OnHovered`
  (params (Selector :type "/DynamicalSystems/Blueprints/BP_InteractableSelector Object Reference"))
  (`TextRenderComponent.SetTextRenderColor` (`self.TextRender`) (`self.HoveredColor`)))

(event `self.BP_Interactable.OnUnhovered`
  (params (Selector :type "/DynamicalSystems/Blueprints/BP_InteractableSelector Object Reference"))
  (`TextRenderComponent.SetTextRenderColor` (`self.TextRender`) (`self.NormalColor`)))

(fn `UserConstructionScript`
  (`TextRenderComponent.SetTextRenderColor` (`self.TextRender`) (`self.NormalColor`)))