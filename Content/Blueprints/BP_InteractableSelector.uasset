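; Selector actor that detects the BP_Interactable component on the object it points at and lets it be interacted with.
; A looping timer at SampleRate drives sampling, which line-traces along the actor's forward vector against a single object type.
; The result updates the cached hovered component, sending hover and unhover notifications when the target changes or is lost.
; TryInteraction calls Interact on the cached component, passing the selector.
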(event `self.ReceiveBeginPlay`
  (if (> (`self.SampleRate`) 0.0)
    (`KismetSystemLibrary.K2_SetTimerDelegate` (`|CreateDelegate` :!event `PerformSampling`) (`self.SampleRate`) true)))

(event `PerformSampling`
  (bind _returnvalue (`self.K2_GetActorLocation`))
  (bind (_outhit _returnvalue_2) (`KismetSystemLibrary.LineTraceSingleForObjects` :`Start` _returnvalue :`End` (+ _returnvalue (* (`self.GetActorForwardVector`) (`self.Sample Distance`))) :`ObjectTypes` (`|MakeArray` "ObjectTypeQuery8" :!type "EObjectTypeQuery Enum") :`DrawTime` (`self.SampleRate`)))
  (if _returnvalue_2
    (bind _returnvalue_3 (`self.GetComponentByClass` (`.HitActor` (`GameplayStatics.BreakHitResult` _outhit)) "/DynamicalSystems/Blueprints/ActorComponents/BP_Interactable.BP_Interactable_C"))
    (`/Engine/EditorBlueprintResources/StandardMacros.IsValid` _returnvalue_3
      (:`Is Valid`
        (`self.CacheCurrentlyHovered` _returnvalue_3))
      (:`Is Not Valid`
        ;[0.1827 0.152 1] We didn't hit anything relevant, but unhover currently hovered object anyway
        (`self.CacheCurrentlyHovered` null :!label _label)))
    (else
      (goto _label))))

(event `CacheCurrentlyHovered`
  (params (incoming :type "/DynamicalSystems/Blueprints/ActorComponents/BP_Interactable Object Reference"))
  (bind _currentlyhoveredactor (`self.CurrentlyHoveredActor`))
  (`/Engine/EditorBlueprintResources/StandardMacros.IsValid` incoming
    (:`Is Valid`
      (if (!= incoming (`self.CurrentlyHoveredActor`))
        (`/DynamicalSystems/Blueprints/ActorComponents/BP_Interactable.OnSelectorHovered` incoming self)
        (`/Engine/EditorBlueprintResources/StandardMacros.IsValid` _currentlyhoveredactor :!label _label_2
          (:`Is Valid`
            (`/DynamicalSystems/Blueprints/ActorComponents/BP_Interactable.OnSelectorUnhovered` _currentlyhoveredactor self))
          (:`Is Not Valid`
            _))
        (set `self.CurrentlyHoveredActor` incoming)))
    (:`Is Not Valid`
      (goto _label_2))))

(event `TryInteraction`
  (bind (_isvalid _interactable) (`self.GetCurrentlyHoveredActor`))
  (if _isvalid
    (`/DynamicalSystems/Blueprints/ActorComponents/BP_Interactable.Interact` _interactable self)))

(fn `GetCurrentlyHoveredActor`
  (returns (IsValid :type Boolean) (Interactable :type "/DynamicalSystems/Blueprints/ActorComponents/BP_Interactable Object Reference") (Actor :type "Actor Object Reference"))
  (bind _currentlyhoveredactor (`self.CurrentlyHoveredActor`))
  (if (`KismetSystemLibrary.IsValid` (`self.CurrentlyHoveredActor`))
    (return true _currentlyhoveredactor (`ActorComponent.GetOwner` _currentlyhoveredactor))
    (else
      (return false null null))))

(fn `GetPlayer`
  (returns (Controller :type "/DynamicalSystems/FullBodyIK/Blueprints/IK_VR_Player Object Reference"))
  (bind _asik_vr_player (cast `/DynamicalSystems/FullBodyIK/Blueprints/IK_VR_Player` (`GameplayStatics.GetPlayerController` 0)))
  (return _asik_vr_player))

(fn `UserConstructionScript`)