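; BP_Interactable is an actor component that lets its owning actor be hovered and interacted with by a Selector.
; Its hover, unhover and interact events relay the Selector through matching OnHovered, OnUnhovered and OnInteracted dispatchers.
; OverrideCollidersType switches the owner's query-enabled shape components to the GameTraceChannel2 object type, though nothing in this file calls it.
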(event `OnSelectorHovered`
  (params (Selector :type "/DynamicalSystems/Blueprints/BP_InteractableSelector Object Reference"))
  (`self.OnHovered` Selector))

(event `OnSelectorUnhovered`
  (params (Selector :type "/DynamicalSystems/Blueprints/BP_InteractableSelector Object Reference"))
  (`self.OnUnhovered` Selector))

(event `Interact`
  (params (Selector :type "/DynamicalSystems/Blueprints/BP_InteractableSelector Object Reference"))
  (`self.OnInteracted` Selector))

(fn `OverrideCollidersType`
  (for _array_element (`Actor.K2_GetComponentsByClass` (`self.GetOwner`) "/Script/Engine.ShapeComponent")
    (if (`PrimitiveComponent.K2_IsQueryCollisionEnabled` _array_element)
      (`PrimitiveComponent.SetCollisionObjectType` _array_element "ECC_GameTraceChannel2"))))