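; BP_SlidingSumWindow is an actor component, per its folder, that keeps a per-index running sum over recently pushed arrays.
; Each push stores the array in a struct stack and updates SumOfArrays incrementally, adding new values and subtracting the oldest entry's, even while filling.
; The oldest entry is dropped once the push count exceeds WindowSize.
; A change in array length clears the stack and resizes the sums.
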(event `PushArrayToStack`
  (params (`Input Array` :type "Array of Float (double-precision)"))
  (bind _returnvalue (`KismetArrayLibrary.Array_Length` `Input Array`))
  (bind _sumofarrays (`self.SumOfArrays`))
  (if (!= _returnvalue (`self.LastArraySize`))
    (`self.ClearStack`)
    (`KismetArrayLibrary.Array_Resize` (`self.InputArray`) _returnvalue)
    (`KismetArrayLibrary.Array_Resize` (`self.SumOfArrays`) _returnvalue))
  (bind _output_get (set `self.InputArray` `Input Array`))
  (`KismetArrayLibrary.Array_Add` (`self.Input Struct`) (make `/DynamicalSystems/Structs/ArrayWindowStruct` _output_get))
  (for (_array_element _array_index) (`self.InputArray`)
    (`KismetArrayLibrary.Array_Set` _sumofarrays _array_index (- (+ _array_element (`KismetArrayLibrary.Array_Get` _sumofarrays _array_index)) (`KismetArrayLibrary.Array_Get` (`.InputArray_3_3C6BDDA34638D6F746658E92E9E9D12E` (break `/DynamicalSystems/Structs/ArrayWindowStruct` (`KismetArrayLibrary.Array_Get` (`self.Input Struct`)))) _array_index))))
  (bind _result (`/Engine/EditorBlueprintResources/StandardMacros.IncrementInt` (`self.CurrentIndex`))
    (:`  `
      (if (> _result (`self.WindowSize`))
        (`KismetArrayLibrary.Array_Remove` (`self.Input Struct`)))
      (set `self.LastArraySize` (`KismetArrayLibrary.Array_Length` (`self.InputArray`))))))

(event `ClearStack`
  (`KismetArrayLibrary.Array_Clear` (`self.Input Struct`))
  (`KismetArrayLibrary.Array_Clear` (`self.SumOfArrays`))
  (`KismetArrayLibrary.Array_Clear` (`self.InputArray`))
  (set `self.CurrentIndex` 0)
  (set `self.LastArraySize` 0))