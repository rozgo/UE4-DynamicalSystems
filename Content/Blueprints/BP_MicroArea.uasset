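; Interactable micro area that teleports the interacting player into it at a shrunken scale.
; On interaction, it gets the player from the Selector and calls TeleportTo with Shrink enabled, using the destination returned by PickTeleportLocation, which is the TeleportationLocation variable.
; The construction script adds a box collider sized by ColliderExtents on a custom object channel, unless UseCustomCollision is set.
; Hover events are empty.
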(event `self.BP_Interactable.OnHovered`
  (params (Selector :type "/DynamicalSystems/Blueprints/BP_InteractableSelector Object Reference")))

(event `self.BP_Interactable.OnUnhovered`
  (params (Selector :type "/DynamicalSystems/Blueprints/BP_InteractableSelector Object Reference")))

(event `self.BP_Interactable.OnInteracted`
  (params (Selector :type "/DynamicalSystems/Blueprints/BP_InteractableSelector Object Reference"))
  (bind _location (`self.PickTeleportLocation`))
  (`/DynamicalSystems/FullBodyIK/Blueprints/IK_VR_Player.TeleportTo` (`/DynamicalSystems/Blueprints/BP_InteractableSelector.GetPlayer` Selector) _location true))

(fn `PickTeleportLocation`
  (returns (Location :type "Vector Structure"))
  (return (`self.TeleportationLocation`)))

(fn `UserConstructionScript`
  (if (not (`self.UseCustomCollision`))
    (bind _returnvalue (`AddComponent|NODE_AddBoxComponent-0` :`RelativeTransform` (`KismetMathLibrary.MakeTransform` (0.0 0.0 0.0))))
    (`BoxComponent.SetBoxExtent` _returnvalue (`self.ColliderExtents`) true)
    (`PrimitiveComponent.SetCollisionObjectType` _returnvalue "ECC_GameTraceChannel2")))