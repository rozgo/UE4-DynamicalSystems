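; BP_HintBubble is an actor that displays a hint as 3D text, turned to face a target component.
; The construction script copies the Text variable into the TextRender component.
; Each Tick, while LookAt is valid, it rotates the whole actor toward that component's world location using a look-at rotation.
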(event `self.ReceiveTick`
  (params (DeltaSeconds :type "Float (single-precision)"))
  (bind _lookat (`self.LookAt`))
  (`/Engine/EditorBlueprintResources/StandardMacros.IsValid` _lookat
    (:`Is Valid`
      (`self.K2_SetActorRotation` (`KismetMathLibrary.FindLookAtRotation` (`self.K2_GetActorLocation`) (`SceneComponent.K2_GetComponentLocation` _lookat))))))

(fn `UserConstructionScript`
  (`TextRenderComponent.K2_SetText` (`self.TextRender`) (`KismetTextLibrary.Conv_StringToText` (`self.Text`))))