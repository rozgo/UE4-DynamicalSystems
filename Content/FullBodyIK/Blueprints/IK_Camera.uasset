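; IK_Camera is a VR camera Blueprint in the FullBodyIK folder that adjusts tracking origin height per headset runtime.
; SetVRHeightOffset moves VROrigin vertically, subtracting the given offset from a base height that is raised only for SteamVR.
; BeginPlay applies this with a zero offset when the HMD device is SteamVR, leaving other devices untouched at startup.
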(event `self.ReceiveBeginPlay`
  (if (== (`HeadMountedDisplayFunctionLibrary.GetHMDDeviceName`) "SteamVR")
    (`self.SetVRHeightOffset` 0.0)))

(fn `SetVRHeightOffset`
  (params (`VR Offset` :type "Float (double-precision)"))
  (locals (DefaultOffset :type "Float (double-precision)"))
  (`SceneComponent.K2_SetRelativeLocation` (`self.VROrigin`) (`KismetMathLibrary.MakeVector` 0.0 0.0 (- (select `bool` (== (`HeadMountedDisplayFunctionLibrary.GetHMDDeviceName`) "SteamVR") :`true` 170.0 :!type "Float (single-precision)") `VR Offset`)) false false))

(fn `UserConstructionScript`)