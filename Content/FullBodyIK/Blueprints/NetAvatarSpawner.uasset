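; Spawner actor that creates networked full-body IK player avatars when the NetClient reports one missing.
; Each Tick it polls NetClient's MissingAvatar ID, spawns an IK_Net_Player regardless of collision, copies the ID into its NetAvatar component, then resets the pending ID.
; It also binds to NetClient's voice activity message on BeginPlay, only printing the received value to screen.
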(event `self.ReceiveBeginPlay`
  (add `NetClient.OnVoiceActivityMsg` (`self.NetClient`) (delegate `OnVoiceActivityMsg_Event_0`)))

(event `OnVoiceActivityMsg_Event_0`
  (params (NetId :type Integer) (Value :type "Float (double-precision)"))
  (`KismetSystemLibrary.PrintString` (`KismetStringLibrary.Conv_DoubleToString` Value)))

(event `self.ReceiveTick`
  (params (DeltaSeconds :type "Float (single-precision)"))
  (bind _netclient (`self.NetClient`))
  (bind _missingavatar (`NetClient.MissingAvatar` _netclient))
  (if (>= _missingavatar 0)
    (bind _returnvalue (`|SpawnActorFromClass` "/DynamicalSystems/FullBodyIK/Blueprints/IK_Net_Player.IK_Net_Player_C" (`KismetMathLibrary.MakeTransform` (0.0 0.0 0.0)) "AlwaysSpawn" "OverrideRootScale" null null))
    (set `NetAvatar.NetID` _missingavatar (`self.GetComponentByClass` _returnvalue "/Script/DynamicalSystems.NetAvatar"))
    (set `NetClient.MissingAvatar` -1 _netclient)))

(fn `UserConstructionScript`)