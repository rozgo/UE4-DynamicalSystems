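; IK_MotionController is the visual motion controller actor for the full-body IK VR pawn.
; Its construction script casts its parent actor to IK_Pawn and uses the pawn's Device setting to pick the Oculus Rift or HTC Vive mesh from the MotionController array.
; It scales the mesh on Y by Flip, which allows mirroring, and has no runtime logic.
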(event `self.ReceiveBeginPlay`)

(fn `UserConstructionScript`
  (bind _staticmesh (`self.StaticMesh`))
  (bind _asik_pawn (cast `/DynamicalSystems/FullBodyIK/Blueprints/IK_Pawn` (`self.GetParentActor`)))
  (if (select `/DynamicalSystems/FullBodyIK/Miscellaneous/E_ListDevice` (`/DynamicalSystems/FullBodyIK/Blueprints/IK_Pawn.Device` _asik_pawn) :`NewEnumerator0` true)
    (set `self.Select` 1)
    (else
      (set `self.Select` 0)))
  (`StaticMeshComponent.SetStaticMesh` _staticmesh (`|GetArrayItem` (`self.MotionController`) (`self.Select`)))
  (`SceneComponent.SetRelativeScale3D` _staticmesh (`KismetMathLibrary.MakeVector` 1.0 (`self.Flip`) 1.0)))