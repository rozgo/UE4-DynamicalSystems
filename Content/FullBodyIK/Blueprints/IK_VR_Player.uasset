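; VR player actor that drives a full-body IK avatar and feeds its pose to a networked avatar.
; On BeginPlay it links NetAvatar to the NetClient, spawns separate IK_Pawn and IK_Camera actors, and makes the camera the view target.
; Tick moves and turns the camera rig from input, copies headset and controller transforms to pawn and NetAvatar, and colors the body by network ID.
; CalibrateHeight sets body height from the headset.
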(event `self.ReceiveBeginPlay`
  (bind _ik_camera (`self.IK_Camera`))
  (`|ExecutionSequence`
    (:`then_0`
      (bind _outactors (`GameplayStatics.GetAllActorsOfClass` "/Script/DynamicalSystems.NetClient"))
      (set `NetAvatar.NetClient` (`|GetArrayItem` _outactors) (`self.NetAvatar`)))
    (:`then_1`
      (bind _returnvalue (`|SpawnActorFromClass` "/DynamicalSystems/FullBodyIK/Blueprints/IK_Pawn.IK_Pawn_C" (`KismetMathLibrary.MakeTransform` (0.0 0.0 0.0)) "AlwaysSpawn" "OverrideRootScale" null null))
      (bind _output_get (set `self.IK_Pawn` _returnvalue))
      (bind _returnvalue_2 (`|SpawnActorFromClass` "/DynamicalSystems/FullBodyIK/Blueprints/IK_Camera.IK_Camera_C" (`KismetMathLibrary.MakeTransform` (0.0 0.0 0.0)) "AlwaysSpawn" "OverrideRootScale" null null))
      (set `self.IK_Camera` _returnvalue_2)
      (`self.SetOwner` (`ChildActorComponent.ChildActor` (`/DynamicalSystems/FullBodyIK/Blueprints/IK_Pawn.ChildHMD` (`self.IK_Pawn`))) _ik_camera)
      (`self.SetViewTargetWithBlend` self _ik_camera 0.0 "VTBlend_Linear" 0.0 false)
      (`HeadMountedDisplayFunctionLibrary.SetTrackingOrigin` "Floor")
      (`HeadMountedDisplayFunctionLibrary.ResetOrientationAndPosition` 0.0))))

(event `self.ReceiveTick`
  (params (DeltaSeconds :type "Float (single-precision)"))
  (bind _ik_pawn (`self.IK_Pawn`))
  (bind _netavatar (`self.NetAvatar`))
  (bind _netavatar_2 (`self.NetAvatar`))
  (bind _netavatar_3 (`self.NetAvatar`))
  (bind _netavatar_4 (`self.NetAvatar`))
  (bind _defaultsceneroot (`/DynamicalSystems/FullBodyIK/Blueprints/IK_Camera.DefaultSceneRoot` (`self.IK_Camera`)))
  (bind _defaultsceneroot_2 (`/DynamicalSystems/FullBodyIK/Blueprints/IK_Camera.DefaultSceneRoot` (`self.IK_Camera`)))
  (bind _defaultsceneroot_3 (`/DynamicalSystems/FullBodyIK/Blueprints/IK_Pawn.DefaultSceneRoot` (`self.IK_Pawn`)))
  (bind _returnvalue (`SceneComponent.K2_GetComponentToWorld` (`/DynamicalSystems/FullBodyIK/Blueprints/IK_Camera.Camera` (`self.IK_Camera`))))
  (bind (_returnvalue_location _returnvalue_rotation) (`KismetMathLibrary.BreakTransform` (`SceneComponent.K2_GetComponentToWorld` (`/DynamicalSystems/FullBodyIK/Blueprints/IK_Pawn.DefaultSceneRoot` (`self.IK_Pawn`)))))
  (bind _returnvalue_2 (`KismetMathLibrary.ComposeTransforms` (`SceneComponent.GetRelativeTransform` (`self.MotionControllerR`)) (`SceneComponent.K2_GetComponentToWorld` (`/DynamicalSystems/FullBodyIK/Blueprints/IK_Camera.VROrigin` (`self.IK_Camera`)))))
  (bind _returnvalue_3 (`KismetMathLibrary.ComposeTransforms` (`SceneComponent.GetRelativeTransform` (`self.MotionControllerL`)) (`SceneComponent.K2_GetComponentToWorld` (`/DynamicalSystems/FullBodyIK/Blueprints/IK_Camera.VROrigin` (`self.IK_Camera`)))))
  (`/Engine/EditorBlueprintResources/StandardMacros.IsValid` _ik_pawn
    (:`Is Valid`
      (`|ExecutionSequence`
        (:`then_0`
          ;[1 1 1] Motion Controlled Locomotion
          (`SceneComponent.K2_SetWorldLocation` _defaultsceneroot (+ (`SceneComponent.K2_GetComponentLocation` _defaultsceneroot_2) (+ (* (`SceneComponent.GetRightVector` _defaultsceneroot_3) (* DeltaSeconds (* (`self.GetInputAxisValue`) -100.0))) (* (`SceneComponent.GetForwardVector` _defaultsceneroot_3) (* DeltaSeconds (* (`self.GetInputAxisValue`) -100.0))))) false false)
          (`SceneComponent.K2_SetWorldRotation` _defaultsceneroot (`KismetMathLibrary.ComposeRotators` (`SceneComponent.K2_GetComponentRotation` _defaultsceneroot_2) (`KismetMathLibrary.MakeRotator` 0.0 0.0 (* (`self.GetInputAxisValue`) 1.0))) false false))
        (:`then_1`
          (`SceneComponent.K2_SetWorldTransform` (`/DynamicalSystems/FullBodyIK/Blueprints/IK_Pawn.ChildMotionControllerL` (`self.IK_Pawn`)) _returnvalue_3 false false)
          (`SceneComponent.K2_SetWorldTransform` (`/DynamicalSystems/FullBodyIK/Blueprints/IK_Pawn.ChildMotionControllerR` (`self.IK_Pawn`)) _returnvalue_2 false false)
          (`SceneComponent.K2_SetWorldTransform` (`/DynamicalSystems/FullBodyIK/Blueprints/IK_Pawn.ChildHMD` (`self.IK_Pawn`)) _returnvalue false false))
        (:`then_2`
          (set `NetAvatar.LocationHandL` (.location _returnvalue_3) _netavatar_3)
          (set `NetAvatar.RotationHandL` (.rotation _returnvalue_3) _netavatar_3)
          (set `NetAvatar.LocationHandR` (.location _returnvalue_2) _netavatar_4)
          (set `NetAvatar.RotationHandR` (.rotation _returnvalue_2) _netavatar_4)
          (set `NetAvatar.LocationHMD` (.location _returnvalue) _netavatar_2)
          (set `NetAvatar.RotationHMD` (.rotation _returnvalue) _netavatar_2)
          (set `NetAvatar.Location` _returnvalue_location _netavatar)
          (set `NetAvatar.Rotation` _returnvalue_rotation _netavatar))
        (:`then_3`
          (`/DynamicalSystems/FullBodyIK/Blueprints/IK_Pawn.SetBodyColor` _ik_pawn (`KismetMathLibrary.HSVToRGB` (/ (`KismetMathLibrary.Conv_IntToDouble` (`NetAvatar.NetID` (`self.NetAvatar`))) 20.0) 0.7 0.5)))))))

(event `InputAction|CalibrateHeight`
  (params (Key :type "Key Structure"))
  (bind (_returnvalue_location _returnvalue_rotation) (`KismetMathLibrary.BreakTransform` (`SceneComponent.K2_GetComponentToWorld` (`/DynamicalSystems/FullBodyIK/Blueprints/IK_Camera.Camera` (`self.IK_Camera`)))))
  (:`Pressed`
    (`/Engine/EditorBlueprintResources/StandardMacros.IsValid` (`self.IK_Pawn`)
      (:`Is Valid`
        (bind _output_get (set `/DynamicalSystems/FullBodyIK/Blueprints/IK_Pawn.Height` (`KismetMathLibrary.FMax` (- (.z (.location (`SceneComponent.K2_GetComponentToWorld` (`/DynamicalSystems/FullBodyIK/Blueprints/IK_Camera.Camera` (`self.IK_Camera`))))) (`/DynamicalSystems/FullBodyIK/Blueprints/IK_Pawn.Floor` (`self.IK_Pawn`)))) (`self.IK_Pawn`)))
        (`KismetSystemLibrary.DrawDebugString` (+ _returnvalue_location (* (`KismetMathLibrary.GetForwardVector` _returnvalue_rotation) 100.0)) (`KismetTextLibrary.Conv_TextToString` (`|FormatText` "Calibrate Height: {Float}" _output_get)) null (struct :`R` 1.0 :`G` 0.535105 :`A` 1.0) 3.0)))))

(fn `UserConstructionScript`)