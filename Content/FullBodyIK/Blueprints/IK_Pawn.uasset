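; VR pawn that drives a full-body IK avatar from headset and motion controller transforms.
; Each tick it estimates center of mass on a cubic Bezier between HMD and pawn root, shaped by their height-normalized distance, and debug-draws the curve.
; The root eases toward that point in XY and toward headset yaw.
; IK_Animation receives offset head and hand transforms, center of mass, height, floor and a PID-style controller's output as velocity.
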(event `self.ReceiveBeginPlay`
  (`|ExecutionSequence`
    (:`then_1`
      (bind _asik_character (cast `/DynamicalSystems/FullBodyIK/Characters/Mannequin/IK_Character` (`ChildActorComponent.ChildActor` (`self.ChildCharacter`))))
      (set `self.Character` _asik_character)
      (bind _asik_animation (cast `/DynamicalSystems/FullBodyIK/Characters/Mannequin/Blueprints/IK_Animation` (`SkeletalMeshComponent.GetAnimInstance` (`/DynamicalSystems/FullBodyIK/Characters/Mannequin/IK_Character.SkeletalMesh` (`self.Character`)))))
      (set `self.AnimInstance` _asik_animation)
      (`|ExecutionSequence`
        (:`then_0`
          (bind _returnvalue (`PrimitiveComponent.CreateDynamicMaterialInstance` (`/DynamicalSystems/FullBodyIK/Characters/Mannequin/IK_Character.SkeletalMesh` (`self.Character`)) 0 "/DynamicalSystems/FullBodyIK/Characters/Mannequin/Materials/MI_AbstractBody.MI_AbstractBody"))
          (set `self.BodyMaterial` _returnvalue))
        (:`then_1`
          (bind _returnvalue_2 (`PrimitiveComponent.CreateDynamicMaterialInstance` (`/DynamicalSystems/FullBodyIK/Characters/Mannequin/IK_Character.SkeletalMesh` (`self.Character`)) 1 "/DynamicalSystems/FullBodyIK/Characters/Mannequin/Materials/MI_AbstractBody.MI_AbstractBody"))
          (set `self.LogoMaterial` _returnvalue_2))))
    (:`then_2`
      (`self.SetupTransforms`))))

(event `self.ReceiveTick`
  (params (DeltaSeconds :type "Float (single-precision)"))
  (bind _velocityarrowhmd (`self.VelocityArrowHMD`))
  (bind _animinstance (`self.AnimInstance`))
  (bind _defaultsceneroot (`self.DefaultSceneRoot`))
  (bind (_returnvalue_x _returnvalue_y _returnvalue_z) (`KismetMathLibrary.BreakVector` (`SceneComponent.K2_GetComponentLocation` _defaultsceneroot)))
  (bind (_returnvalue_x_2 _returnvalue_y_2 _returnvalue_z_2) (`KismetMathLibrary.BreakVector` (`SceneComponent.GetSocketLocation` (`/DynamicalSystems/FullBodyIK/Characters/Mannequin/IK_Character.SkeletalMesh` (`self.Character`)) "foot_r")))
  (bind _returnvalue (`self.K2_GetActorLocation` (`ChildActorComponent.ChildActor` (`self.ChildHMD`))))
  (bind (_returnvalue_x_3 _returnvalue_y_3) (`KismetMathLibrary.BreakVector` (`SceneComponent.K2_GetComponentLocation` (`/DynamicalSystems/FullBodyIK/Blueprints/IK_Transform.DefaultSceneRoot` (`self.CenterOfMass`)))))
  (bind _returnvalue_2 (- _returnvalue (`self.LastLocationHMD`)))
  (`|ExecutionSequence`
    (:`then_0`
      (bind _output_get (set `/DynamicalSystems/FullBodyIK/Characters/Mannequin/Blueprints/IK_Animation.Height` (`self.Height`) _animinstance))
      (set `/DynamicalSystems/FullBodyIK/Characters/Mannequin/Blueprints/IK_Animation.Floor` (`self.Floor`) _animinstance)
      (`SceneComponent.SetWorldScale3D` (`/DynamicalSystems/FullBodyIK/Characters/Mannequin/IK_Character.SkeletalMesh` (`self.Character`)) (`KismetMathLibrary.Conv_DoubleToVector` (/ _output_get 160.0))))
    (:`then_1`
      (if (> (`KismetMathLibrary.VSize` _returnvalue_2) 0.1)
        (`SceneComponent.K2_SetWorldRotation` _velocityarrowhmd (`KismetMathLibrary.MakeRotFromX` _returnvalue_2) false false)
        (`SceneComponent.K2_SetWorldLocation` _velocityarrowhmd (+ (`SceneComponent.K2_GetComponentLocation` (`/DynamicalSystems/FullBodyIK/Blueprints/IK_Transform.DefaultSceneRoot` (`self.CenterOfMass`))) (0.0 0.0 20.0)) false false)))
    (:`then_2`
      (`self.UpdateTransforms`))
    (:`then_3`
      (`self.ApplyTransforms`))
    (:`then_4`
      (set `self.LastLocationHMD` _returnvalue))
    (:`then_6`
      (`SceneComponent.K2_SetWorldLocation` (`self.DefaultSceneRoot`) (`KismetMathLibrary.VInterpTo` (`SceneComponent.K2_GetComponentLocation` _defaultsceneroot) (`KismetMathLibrary.MakeVector` _returnvalue_x_3 _returnvalue_y_3 _returnvalue_z) DeltaSeconds 5.0) false false)
      (`SceneComponent.K2_SetWorldRotation` (`self.DefaultSceneRoot`) (`KismetMathLibrary.RInterpTo` (`SceneComponent.K2_GetComponentRotation` (`self.DefaultSceneRoot`)) (`KismetMathLibrary.MakeRotator` 0.0 0.0 (+ (.yaw (.rotation (`self.ClampUpTransform` (`self.GetTransform` (`ChildActorComponent.ChildActor` (`self.ChildHMD`)))))) -90.0)) DeltaSeconds 3.0) false false))
    (:`then_7`
      (`|ExecutionSequence`
        (:`then_1`
          (set `self.FootRPrev` _returnvalue_z_2))))))

(fn `SetBodyColor`
  (params (Color :type "LinearColor Structure"))
  (`MaterialInstanceDynamic.SetVectorParameterValue` (`self.BodyMaterial`) "AvatarColor" Color)
  (`MaterialInstanceDynamic.SetVectorParameterValue` (`self.LogoMaterial`) "AvatarColor" Color))

(fn `UserConstructionScript`)