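; Debug driver that feeds simulated VR tracking motion to the full-body IK pawn, IK_Pawn.
; On BeginPlay it grabs the first IK_Pawn in the level, then every tick moves its left controller, right controller and HMD components.
; Each follows its own time-based sine/cosine circle around a fixed world-space offset, at differing speeds and planes.
; Logic for possession, leg calibration montage and view-target blending is present but never runs.
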(event `self.ReceiveBeginPlay`
  (bind _outactors (`GameplayStatics.GetAllActorsOfClass` "/DynamicalSystems/FullBodyIK/Blueprints/IK_Pawn.IK_Pawn_C"))
  (bind _output_get (set `self.IK_Pawn` (`|GetArrayItem` _outactors))))

(event `self.ReceiveTick`
  (params (DeltaSeconds :type "Float (single-precision)"))
  (`/Engine/EditorBlueprintResources/StandardMacros.IsValid` (`self.IK_Pawn`)
    (:`Is Valid`
      (`|ExecutionSequence`
        (:`then_0`
          (`self.TestHandL`))
        (:`then_1`
          (`self.TestHandR`))
        (:`then_2`
          (`self.TestHMD`))))))

(fn `TestHandL`
  (bind _returnvalue (* (`KismetSystemLibrary.GetGameTimeInSeconds`) 180.0))
  (`SceneComponent.K2_SetWorldLocation` (`/DynamicalSystems/FullBodyIK/Blueprints/IK_Pawn.ChildMotionControllerL` (`self.IK_Pawn`)) (+ (* (`KismetMathLibrary.MakeVector` 0.0 (`KismetMathLibrary.DegCos` _returnvalue) (`KismetMathLibrary.DegSin` _returnvalue)) 10.0) (`KismetMathLibrary.MakeVector` 60.0 0.0 140.0)) false false))

(fn `TestHandR`
  (bind _returnvalue (* (`KismetSystemLibrary.GetGameTimeInSeconds`) 100.0))
  (`SceneComponent.K2_SetWorldLocation` (`/DynamicalSystems/FullBodyIK/Blueprints/IK_Pawn.ChildMotionControllerR` (`self.IK_Pawn`)) (+ (* (`KismetMathLibrary.MakeVector` (`KismetMathLibrary.DegSin` _returnvalue) 0.0 (`KismetMathLibrary.DegCos` _returnvalue)) 10.0) (`KismetMathLibrary.MakeVector` -30.0 20.0 180.0)) false false))

(fn `TestHMD`
  (bind _returnvalue (* (`KismetSystemLibrary.GetGameTimeInSeconds`) 40.0))
  (`SceneComponent.K2_SetWorldLocation` (`/DynamicalSystems/FullBodyIK/Blueprints/IK_Pawn.ChildHMD` (`self.IK_Pawn`)) (+ (* (`KismetMathLibrary.MakeVector` (`KismetMathLibrary.DegSin` _returnvalue) (`KismetMathLibrary.DegCos` _returnvalue)) 50.0) (`KismetMathLibrary.MakeVector` 0.0 20.0 170.0)) false false))

(fn `UserConstructionScript`)